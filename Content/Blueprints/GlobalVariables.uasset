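; GlobalVariables is an actor holding the game's population and density map grids, plus helpers that edit population and record the slot awaiting placement.
; Data table columns are flattened into float arrays indexed by row and column, with population appended in both the construction script and BeginPlay.
; PopulationMovementAction draws population into a tile from two neighbour rings using per-ring factors and a tile cap.
; DecreasePopulation subtracts a given amount from one tile.
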(event `self.ReceiveBeginPlay`
  (`|ExecutionSequence`
    (:`then_0`
      ;[1 1 1] Create array for density [with example of how to use it]
      (for _index (range 1 91)
        (bind _returnvalue (`DataTableFunctionLibrary.GetDataTableColumnAsString` "/Game/Blueprints/DataRelated/CSVs/MAP_densityStructured.MAP_densityStructured" (`KismetStringLibrary.Conv_StringToName` (`KismetStringLibrary.Conv_IntToString` _index))))
        (for _array_element _returnvalue
          (`KismetArrayLibrary.Array_Add` (`self.DensityArray`) (`KismetStringLibrary.Conv_StringToDouble` _array_element))))
      (bind _value (`self.GetPopData` (`self.row`) (`self.column`) (`self.DensityArray`))))
    (:`then_1`
      ;[1 1 1] Create array for population [with example how to use it]
      (for _index_2 (range 1 91)
        (bind _returnvalue_2 (`DataTableFunctionLibrary.GetDataTableColumnAsString` "/Game/Blueprints/DataRelated/CSVs/MAP_population_structured_1Mdivided.MAP_population_structured_1Mdivided" (`KismetStringLibrary.Conv_StringToName` (`KismetStringLibrary.Conv_IntToString` _index_2))))
        (for _array_element_2 _returnvalue_2
          (`KismetArrayLibrary.Array_Add` (`self.PopulationArray`) (`KismetStringLibrary.Conv_StringToDouble` _array_element_2))))
      (bind _value_2 (`self.GetPopData` (`self.row`) (`self.column`) (`self.PopulationArray`))))
    (:`then_2`
      ;[1 1 1] just test to see population, PopTest to be removed later as well
      (for _index_3 (range (* 64 90))
        (set `self.PopTest` (+ (`|GetArrayItem` (`self.PopulationArray`) _index_3) (`self.PopTest`))))
      (`KismetSystemLibrary.PrintString` "CURRENT POPULATION")
      (`KismetSystemLibrary.PrintString` (`KismetStringLibrary.Conv_DoubleToString` (`self.PopTest`))))))

(fn `Create Neighbour L1Array`
  (params (Row :type "Float (double-precision)") (Column :type "Float (double-precision)"))
  (returns (NeihgbourL2Array :type "Array of Vector2D Structure"))
  (locals (RowMin1 :type "Float (double-precision)") (RowOryg :type "Float (double-precision)") (RowPlus1 :type "Float (double-precision)") (ColumnMin1 :type "Float (double-precision)") (ColumnOryg :type "Float (double-precision)") (ColumnPlus1 :type "Float (double-precision)"))
  (bind _roworyg (`local.RowOryg`))
  (bind _roworyg_2 (`local.RowOryg`))
  (bind _rowmin1 (`local.RowMin1`))
  (bind _rowplus1 (`local.RowPlus1`))
  (bind _columnoryg (`local.ColumnOryg`))
  (set `local.RowOryg` Row)
  (set `local.ColumnOryg` Column)
  ;[1 1 1] setting helper variables for level 1 neighbours of gether points
  (set `local.RowMin1` (- _roworyg 1.0))
  (set `local.RowPlus1` (+ _roworyg 1.0))
  (set `local.ColumnMin1` (- _columnoryg 1.0))
  (set `local.ColumnPlus1` (+ _columnoryg 1.0))
  (return (`|MakeArray` (`KismetMathLibrary.MakeVector2D` _rowmin1 (`local.ColumnMin1`)) (`KismetMathLibrary.MakeVector2D` _rowmin1 (`local.ColumnOryg`)) (`KismetMathLibrary.MakeVector2D` _rowmin1 (`local.ColumnPlus1`)) (`KismetMathLibrary.MakeVector2D` _roworyg_2 (`local.ColumnMin1`)) (`KismetMathLibrary.MakeVector2D` _roworyg_2 (`local.ColumnPlus1`)) (`KismetMathLibrary.MakeVector2D` _rowplus1 (`local.ColumnOryg`)) (`KismetMathLibrary.MakeVector2D` _rowplus1 (`local.ColumnMin1`)) (`KismetMathLibrary.MakeVector2D` _rowplus1 (`local.ColumnPlus1`)))))

(fn `Create Neighbour L2Array`
  (params (Row :type "Float (double-precision)") (Column :type "Float (double-precision)"))
  (returns (NeihgbourL2Array :type "Array of Vector2D Structure"))
  (locals (RowMin2 :type "Float (double-precision)") (RowMin1 :type "Float (double-precision)") (RowOryg :type "Float (double-precision)") (RowPlus1 :type "Float (double-precision)") (RowPlus2 :type "Float (double-precision)") (ColumnMin2 :type "Float (double-precision)") (ColumnMin1 :type "Float (double-precision)") (ColumnOryg :type "Float (double-precision)") (ColumnPlus1 :type "Float (double-precision)") (ColumnPlus2 :type "Float (double-precision)"))
  (bind _roworyg (`local.RowOryg`))
  (bind _columnmin2 (`local.ColumnMin2`))
  (bind _columnplus2 (`local.ColumnPlus2`))
  (bind _rowplus2 (`local.RowPlus2`))
  (bind _rowmin2 (`local.RowMin2`))
  (bind _columnoryg (`local.ColumnOryg`))
  (set `local.RowOryg` Row)
  (set `local.ColumnOryg` Column)
  ;[1 1 1] setting helper variables for level 1 neighbours of gether points
  (set `local.RowMin2` (- _roworyg 2.0))
  (set `local.RowMin1` (- _roworyg 1.0))
  (set `local.RowPlus1` (+ _roworyg 1.0))
  (set `local.RowPlus2` (+ _roworyg 2.0))
  (set `local.ColumnMin2` (- _columnoryg 2.0))
  (set `local.ColumnMin1` (- _columnoryg 1.0))
  (set `local.ColumnPlus1` (+ _columnoryg 1.0))
  (set `local.ColumnPlus2` (+ _columnoryg 2.0))
  (return (`|MakeArray` (`KismetMathLibrary.MakeVector2D` (`local.RowMin2`) _columnmin2) (`KismetMathLibrary.MakeVector2D` (`local.RowMin1`) _columnmin2) (`KismetMathLibrary.MakeVector2D` (`local.RowOryg`) _columnmin2) (`KismetMathLibrary.MakeVector2D` (`local.RowPlus1`) _columnmin2) (`KismetMathLibrary.MakeVector2D` (`local.RowPlus2`) _columnmin2) (`KismetMathLibrary.MakeVector2D` (`local.RowMin2`) _columnplus2) (`KismetMathLibrary.MakeVector2D` (`local.RowMin1`) _columnplus2) (`KismetMathLibrary.MakeVector2D` (`local.RowOryg`) _columnplus2) (`KismetMathLibrary.MakeVector2D` (`local.RowPlus1`) _columnplus2) (`KismetMathLibrary.MakeVector2D` (`local.RowPlus2`) _columnplus2) (`KismetMathLibrary.MakeVector2D` _rowmin2 (`local.ColumnMin1`)) (`KismetMathLibrary.MakeVector2D` _rowmin2 (`local.ColumnOryg`)) (`KismetMathLibrary.MakeVector2D` _rowmin2 (`local.ColumnPlus1`)) (`KismetMathLibrary.MakeVector2D` _rowplus2 (`local.ColumnMin1`)) (`KismetMathLibrary.MakeVector2D` _rowplus2 (`local.ColumnOryg`)) (`KismetMathLibrary.MakeVector2D` _rowplus2 (`local.ColumnPlus1`)))))

(fn `DecreasePopulation`
  (params (Row :type Integer) (Column :type Integer) (DecreaseInM :type "Float (double-precision)"))
  (bind _index (`self.GetMapArrayIndex` Row Column))
  (bind _value (`self.GetPopData` Row Column (`self.PopulationArray`)))
  (`KismetSystemLibrary.PrintString` (`KismetStringLibrary.Conv_DoubleToString` _value))
  (`KismetArrayLibrary.Array_Set` (`self.PopulationArray`) _index (- _value DecreaseInM))
  (bind _value_2 (`self.GetPopData` Row Column (`self.PopulationArray`)))
  (`KismetSystemLibrary.PrintString` (`KismetStringLibrary.Conv_DoubleToString` _value_2)))

(fn `GetMapArrayIndex`
  (params (Row :type Integer) (Column :type Integer))
  (returns (Index :type Integer))
  (return (- (* Column 64) Row)))

(fn `GetPopData`
  (params (Row :type Integer) (Column :type Integer) (MapArray :type "Array of Float (double-precision)"))
  (returns (Value :type "Float (double-precision)"))
  (return (`|GetArrayItem` MapArray (- (* Column 64) Row))))

(fn `PopulationMovementAction`
  (params (Row :type Integer) (Column :type Integer))
  (locals (InitialPopulation :type "Float (double-precision)") (RowOryg :type "Float (double-precision)" :default 0.0) (ColumnOryg :type "Float (double-precision)" :default 0.0) (NeighbourL1Arr :type "Array of Vector2D Structure") (NeighbourL2Arr :type "Array of Vector2D Structure") (GPPopulation :type "Float (double-precision)" :default 0.0) (NeighbourPopulation :type "Float (double-precision)" :default 0.0) (GP_index :type Integer :default 0) (NeighbourIndex :type Integer :default 0) (TestInitPopL1 :type "Float (double-precision)") (TestInitPopL2 :type "Float (double-precision)") (TestFinalPopL1 :type "Float (double-precision)") (TestFinalPopL2 :type "Float (double-precision)"))
  (bind _returnvalue (- (`self.MaxTilePopulationM`) (`local.GPPopulation`)))
  (bind _returnvalue_2 (- (`self.MaxTilePopulationM`) (`local.GPPopulation`)))
  (bind _returnvalue_3 (+ (`local.GPPopulation`) (`local.NeighbourPopulation`)))
  (bind _returnvalue_4 (+ (`local.GPPopulation`) (`local.NeighbourPopulation`)))
  (bind _returnvalue_5 (- (`local.NeighbourPopulation`) _returnvalue))
  (bind _returnvalue_6 (>= _returnvalue (`local.NeighbourPopulation`)))
  (bind _returnvalue_7 (- (`local.NeighbourPopulation`) _returnvalue_2))
  (bind _returnvalue_8 (>= _returnvalue_2 (`local.NeighbourPopulation`)))
  (bind _returnvalue_9 (+ (`local.GPPopulation`) (* (`local.NeighbourPopulation`) (`self.L1MovementFactor`))))
  (bind _returnvalue_10 (+ (`local.GPPopulation`) (* (`local.NeighbourPopulation`) (`self.L2MovementFactor`))))
  (bind _returnvalue_11 (+ (`local.GPPopulation`) _returnvalue_5))
  (bind _returnvalue_12 (+ (`local.GPPopulation`) _returnvalue_7))
  ;[1 1 1] Setting required Variables
  (bind _index (`self.GetMapArrayIndex` Row Column))
  (set `local.RowOryg` (`KismetMathLibrary.Conv_IntToDouble` Row))
  (set `local.ColumnOryg` (`KismetMathLibrary.Conv_IntToDouble` Column))
  (set `local.GP_index` _index)
  (bind _output_get (set `local.InitialPopulation` (`|GetArrayItem` (`self.PopulationArray`) _index)))
  (set `local.GPPopulation` _output_get)
  (bind _neihgbourl2array (`self.Create Neighbour L1Array` (`local.RowOryg`) (`local.ColumnOryg`)))
  (set `local.NeighbourL1Arr` _neihgbourl2array)
  (bind _neihgbourl2array_2 (`self.Create Neighbour L2Array` (`local.RowOryg`) (`local.ColumnOryg`)))
  (set `local.NeighbourL2Arr` _neihgbourl2array_2)
  (if (< (`local.GPPopulation`) (`self.MaxTilePopulationM`))
    (`|ExecutionSequence`
      (:`then_0`
        ;[1 1 1] Actions on L1 Neigbours - getting initial values for GP Population and Naighbour population and updating them based n L1 Factor
        (for _array_element (`local.NeighbourL1Arr`)
          (if (> (`local.GPPopulation`) (`self.MaxTilePopulationM`))
            (break)
            (else
              (bind _returnvalue_13 (`KismetMathLibrary.FTrunc` (`KismetMathLibrary.BreakVector2D` _array_element)))
              (bind _returnvalue_14 (`KismetMathLibrary.FTrunc` (`.Y` (`KismetMathLibrary.BreakVector2D` _array_element))))
              (bind _value (`self.GetPopData` _returnvalue_13 _returnvalue_14 (`self.PopulationArray`)))
              (set `local.NeighbourPopulation` _value)
              (bind _index_2 (`self.GetMapArrayIndex` _returnvalue_13 _returnvalue_14))
              (bind _output_get_2 (set `local.NeighbourIndex` _index_2))
              (if (== _output_get_2 0)
                _
                (elif (< (`local.NeighbourPopulation`) 0.3)
                  (if _returnvalue_8
                    ;[1 1 1] If Neighbour Pop is smaller than 0.3 than set it to zero and increase GP Pop accordingly
                    (`KismetArrayLibrary.Array_Set` (`self.PopulationArray`) (`local.NeighbourIndex`))
                    (`KismetArrayLibrary.Array_Set` (`self.PopulationArray`) (`local.GP_index`) _returnvalue_3)
                    (set `local.GPPopulation` _returnvalue_3)
                    (else
                      ;[1 1 1] Decrease Neighbour by the ammount missing in GP Coords to Max Population and set GP Population to Max
                      (`KismetArrayLibrary.Array_Set` (`self.PopulationArray`) (`local.NeighbourIndex`) _returnvalue_7 :!label _label)
                      (`KismetArrayLibrary.Array_Set` (`self.PopulationArray`) (`local.GP_index`) _returnvalue_12)
                      (set `local.GPPopulation` _returnvalue_12)))
                  (elif _returnvalue_8
                    ;[1 1 1] Decrease Neighb Pop by L1 Factor and increase GP Population accordingly
                    (`KismetArrayLibrary.Array_Set` (`self.PopulationArray`) (`local.NeighbourIndex`) (* (`local.NeighbourPopulation`) (- 1.0 (`self.L1MovementFactor`))))
                    (`KismetArrayLibrary.Array_Set` (`self.PopulationArray`) (`local.GP_index`) _returnvalue_9)
                    (set `local.GPPopulation` _returnvalue_9)
                    (else
                      (goto _label)))))))))
      (:`then_1`
        ;[1 1 1] Actions on L2 Neigbours - getting initial values for GP Population and Naighbour population and updating them based n L1 Factor
        (for _array_element_2 (`local.NeighbourL2Arr`)
          (if (> (`local.GPPopulation`) (`self.MaxTilePopulationM`))
            (break)
            (else
              (bind _returnvalue_15 (`KismetMathLibrary.FTrunc` (`KismetMathLibrary.BreakVector2D` _array_element_2)))
              (bind _returnvalue_16 (`KismetMathLibrary.FTrunc` (`.Y` (`KismetMathLibrary.BreakVector2D` _array_element_2))))
              (bind _value_2 (`self.GetPopData` _returnvalue_15 _returnvalue_16 (`self.PopulationArray`)))
              (set `local.NeighbourPopulation` _value_2)
              (bind _index_3 (`self.GetMapArrayIndex` _returnvalue_15 _returnvalue_16))
              (bind _output_get_3 (set `local.NeighbourIndex` _index_3))
              (if (== _output_get_3 0)
                _
                (elif (< (`local.NeighbourPopulation`) 0.3)
                  (if _returnvalue_6
                    ;[1 1 1] If Neighbour Pop is smaller than 0.3 than set it to zero and increase GP Pop accordingly
                    (`KismetArrayLibrary.Array_Set` (`self.PopulationArray`) (`local.NeighbourIndex`))
                    (`KismetArrayLibrary.Array_Set` (`self.PopulationArray`) (`local.GP_index`) _returnvalue_4)
                    (set `local.GPPopulation` _returnvalue_4)
                    (else
                      ;[1 1 1] If difference between pop in GP Tile and max Pop is smaller than Neighb Pop, then Decrease Neighbour by the ammount missing in GP Coords to Max Population and set GP Population to Max
                      (`KismetArrayLibrary.Array_Set` (`self.PopulationArray`) (`local.NeighbourIndex`) _returnvalue_5 :!label _label_2)
                      (`KismetArrayLibrary.Array_Set` (`self.PopulationArray`) (`local.GP_index`) _returnvalue_11)
                      (set `local.GPPopulation` _returnvalue_11)))
                  (elif _returnvalue_6
                    ;[1 1 1] Else, Decrease Neighb Pop by L2 Factor and increase GP Population accordingly
                    (`KismetArrayLibrary.Array_Set` (`self.PopulationArray`) (`local.NeighbourIndex`) (* (`local.NeighbourPopulation`) (- 1.0 (`self.L2MovementFactor`))))
                    (`KismetArrayLibrary.Array_Set` (`self.PopulationArray`) (`local.GP_index`) _returnvalue_10)
                    (set `local.GPPopulation` _returnvalue_10)
                    (else
                      (goto _label_2))))))))))))

(fn `UserConstructionScript`
  ;[1 1 1] Create array for population [with example how to use it]
  (for _index (range 1 91)
    (bind _returnvalue (`DataTableFunctionLibrary.GetDataTableColumnAsString` "/Game/Blueprints/DataRelated/CSVs/MAP_population_structured_1Mdivided.MAP_population_structured_1Mdivided" (`KismetStringLibrary.Conv_StringToName` (`KismetStringLibrary.Conv_IntToString` _index))))
    (for _array_element _returnvalue
      (`KismetArrayLibrary.Array_Add` (`self.PopulationArray`) (`KismetStringLibrary.Conv_StringToDouble` _array_element))))
  (bind _value (`self.GetPopData` (`self.row`) (`self.column`) (`self.PopulationArray`))))

(fn `WaitingOnPlacement`
  (params (SlotIndex :type Integer))
  (if (or (`self.PlaceRocket`) (`self.PlaceEP`) (`self.PlaceIT`))
    (set `self.SlotWaitingToBePlaced` SlotIndex)
    (else
      (`KismetSystemLibrary.PrintString` "Nothing to place"))))