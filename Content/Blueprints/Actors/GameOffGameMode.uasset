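; Game mode that tracks Earth's population and feeds the totals to the AI screen widget.
; On BeginPlay, after short delays, it caches the grid, GlobalVariables actor and AiScreen widget, and records the initial population.
; Each tick it re-sums the per-cell population array, updating the widget's Earth and lost counts, with saved people excluded from losses.
; At zero population it only prints a game-over message, with on-screen display disabled.
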(event `self.ReceiveBeginPlay`
  (`KismetSystemLibrary.Delay` 0.2)
  (bind _outactors (`GameplayStatics.GetAllActorsOfClass` "/Game/Blueprints/Actors/MapNavigationSolutions/BP_grid.BP_grid_C"))
  (set `self.Grid` (`|GetArrayItem` _outactors))
  (bind _outactors_2 (`GameplayStatics.GetAllActorsOfClass` "/Game/Blueprints/GlobalVariables.GlobalVariables_C"))
  (set `self.GlobalVariables` (`|GetArrayItem` _outactors_2))
  (bind _population (`self.CountPopulation`))
  (set `self.InitialPopulation` _population)
  (`KismetSystemLibrary.Delay` 0.1)
  (bind _foundwidgets (`WidgetBlueprintLibrary.GetAllWidgetsOfClass` "/Game/Blueprints/UiWidgets/ScreenUI/AiScreen.AiScreen_C"))
  (set `self.AIScreen` (`|GetArrayItem` _foundwidgets)))

(event `self.ReceiveTick`
  (params (DeltaSeconds :type "Float (single-precision)"))
  (bind _population (`self.CountPopulation`))
  (if (<= _population 0.0)
    (`KismetSystemLibrary.PrintString` "GAME OVER" false)
    (else
      (bind _output_get (set `/Game/Blueprints/UiWidgets/ScreenUI/AiScreen.EarthPopulation` _population (`self.AIScreen`)))
      (set `/Game/Blueprints/UiWidgets/ScreenUI/AiScreen.LostPopulation` (- (- (`self.InitialPopulation`) _output_get) (`/Game/Blueprints/UiWidgets/ScreenUI/AiScreen.SavedPopulation` (`self.AIScreen`))) (`self.AIScreen`)))))

(fn `CountPopulation`
  (returns (Population :type "Float (double-precision)"))
  (set `self.CurrentEarthPopulation` 0.0)
  (for _index (range (* (`self.Rows`) (`self.Columns`)))
    (set `self.CurrentEarthPopulation` (+ (`|GetArrayItem` (`/Game/Blueprints/GlobalVariables.PopulationArray` (`self.GlobalVariables`)) _index) (`self.CurrentEarthPopulation`))))
  (return (`self.CurrentEarthPopulation`)))

(fn `GetGrid`
  (returns (Grid :type "/Game/Blueprints/Actors/MapNavigationSolutions/BP_grid Object Reference"))
  (return (`self.Grid`)))

(fn `UserConstructionScript`)