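; Game mode, named for the main menu, that exposes a grid and totals Earth's population.
; GetGrid returns the stored Grid.
; CountPopulation resets CurrentEarthPopulation, sums the GlobalVariables population array over every row-by-column cell, then stores and returns the total.
; BeginPlay and the construction script are empty, so both functions run only when called.
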(event `self.ReceiveBeginPlay`)

(fn `CountPopulation`
  (returns (Population :type "Float (double-precision)"))
  (set `self.CurrentEarthPopulation` 0.0)
  (for _index (range (* (`self.Rows`) (`self.Columns`)))
    (set `self.CurrentEarthPopulation` (+ (`|GetArrayItem` (`/Game/Blueprints/GlobalVariables.PopulationArray` (`self.GlobalVariables`)) _index) (`self.CurrentEarthPopulation`))))
  (return (`self.CurrentEarthPopulation`)))

(fn `GetGrid`
  (returns (Grid :type "/Game/Blueprints/Actors/MapNavigationSolutions/BP_grid Object Reference"))
  (return (`self.Grid`)))

(fn `UserConstructionScript`)